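; BP_Observer is a player-controlled observer that moves and looks around using Enhanced Input with the IMC_Observer mapping context.
; Movement follows the controller's forward and right vectors, scaled down when both axes are pressed.
; A FlipFlop toggle feeds SetInputMode, switching between game-only input and a mouse cursor mode that ignores look and move.
; A test action toggles prompt or sound handling by server type, while SetText is empty and info-widget logic is unwired.
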(event `self.ReceiveBeginPlay`
  (`EnhancedInputSubsystemInterface.AddMappingContext` (pcsubsystem `EnhancedInputLocalPlayerSubsystem` (`GameplayStatics.GetPlayerController` 0)) "/Game/Platform/Input/IMC_Observer.IMC_Observer" 0 (struct)))

(event `EnhancedInput|/Game/Platform/Input/InputAction/IA_Move`
  (params (ActionValue :type "Vector2D Structure") (ElapsedSeconds :type "Float (double-precision)") (TriggeredSeconds :type "Float (double-precision)") (InputAction :type "InputAction Object Reference" :default "/Game/Platform/Input/InputAction/IA_Move.IA_Move"))
  (:`Triggered`
    (`self.AddMovementInput` (`self.GetActorForwardVector` (`self.GetController`)) (`KismetMathLibrary.SelectFloat` (* ActionValue_X 0.5) (* ActionValue_X 0.3) (== ActionValue_Y 0.0)))
    (`self.AddMovementInput` (`self.GetActorRightVector` (`self.GetController`)) (`KismetMathLibrary.SelectFloat` (* ActionValue_Y 0.5) (* ActionValue_Y 0.3) (== ActionValue_X 0.0)))))

(event `EnhancedInput|/Game/Platform/Input/InputAction/IA_Look`
  (params (ActionValue :type "Vector2D Structure") (ElapsedSeconds :type "Float (double-precision)") (TriggeredSeconds :type "Float (double-precision)") (InputAction :type "InputAction Object Reference" :default "/Game/Platform/Input/InputAction/IA_Look.IA_Look"))
  (:`Triggered`
    (`self.AddControllerYawInput` ActionValue_X)
    (`self.AddControllerPitchInput` ActionValue_Y)))

(event `EnhancedInput|/Game/Platform/Input/InputAction/IA_ToggleMouseCursor`
  (params (ActionValue :type Boolean) (ElapsedSeconds :type "Float (double-precision)") (TriggeredSeconds :type "Float (double-precision)") (InputAction :type "InputAction Object Reference" :default "/Game/Platform/Input/InputAction/IA_ToggleMouseCursor.IA_ToggleMouseCursor"))
  (:`Started`
    (bind _isa (`/Engine/EditorBlueprintResources/StandardMacros.FlipFlop`)
      (:`A`
        _)
      (:`B`
        _))
    (`self.SetInputMode` _isa)))

(event `EnhancedInput|/Game/Blueprint/Basic/IA_TEST`
  (params (ActionValue :type Boolean) (ElapsedSeconds :type "Float (double-precision)") (TriggeredSeconds :type "Float (double-precision)") (InputAction :type "InputAction Object Reference" :default "/Game/Blueprint/Basic/IA_TEST.IA_TEST"))
  (:`Started`
    (`|ExecutionSequence`
      (:`then_0`
        (if (`KismetSystemLibrary.IsDedicatedServer`)
          (`SceneComponent.SetVisibility` (`self.PromptText`) false false)
          (else
            (`GameplayStatics.SpawnSound2D` null 1.0 1.0 0.0 null))))
      (:`then_1`
        (`self.SetText` false)))))

(event `press`)

(fn `SetInputMode`
  (params (bGameInput :type Boolean))
  (bind _pc_base (`/Game/Platform/System/BPFL_SystemLib.GetBasePlayerController`))
  (if bGameInput
    (set `PlayerController.bShowMouseCursor` false _pc_base)
    (`WidgetBlueprintLibrary.SetInputMode_GameOnly` _pc_base)
    (`Controller.ResetIgnoreInputFlags` _pc_base)
    (else
      (set `PlayerController.bShowMouseCursor` true _pc_base)
      (`WidgetBlueprintLibrary.SetInputMode_GameAndUIEx` _pc_base null)
      (`Controller.SetIgnoreLookInput` _pc_base true)
      (`Controller.SetIgnoreMoveInput` _pc_base true))))

(fn `SetText`
  (params (Condition :type Boolean)))

(fn `UserConstructionScript`)