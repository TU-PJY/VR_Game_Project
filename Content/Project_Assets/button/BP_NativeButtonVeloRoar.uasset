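; Native button actor that plays a 2D velociraptor squeal whenever its ButtonComp changes state.
; On/Off text is set at BeginPlay on standalone or remote instances, and a LastButtonState RepNotify resyncs button position, color and text.
; RunButton toggles an info widget, voice-over and spawned BP_UMGDisplayVelo at the camera, but its only call in this graph is disconnected.
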(event `self.ReceiveBeginPlay`
  (`self.SetText` (`VRButtonComponent.bButtonState` (`self.ButtonComp`))))

(event `SetText`
  (params (State :type Boolean))
  (bind _textrender (`self.TextRender`))
  (`/Engine/EditorBlueprintResources/ActorMacros.Switch Has Authority`
    (:`Authority`
      (if (`KismetSystemLibrary.IsStandalone`)
        (if State :!label _label
          (`TextRenderComponent.K2_SetText` _textrender (`self.OnText`))
          (else
            (`TextRenderComponent.K2_SetText` _textrender (`self.OffText`))))))
    (:`Remote`
      (goto _label))))

(event `CustomEvent`
  (params (ButtonState :type Boolean) (InteractingActor :type "Actor Object Reference") (InteractingComponent :type "PrimitiveComponent Object Reference")))

(event `self.ButtonComp.OnButtonStateChanged`
  (params (ButtonState :type Boolean) (InteractingActor :type "Actor Object Reference") (InteractingComponent :type "PrimitiveComponent Object Reference"))
  (`GameplayStatics.PlaySound2D` "/Game/TTS_File/velociraptor-squeal-epic-stock-media-1-00-01.velociraptor-squeal-epic-stock-media-1-00-01" 1.0 1.0 0.0 null null))

(fn `OnRep_LastButtonState`
  (bind _lastbuttonstate (`self.LastButtonState`))
  (bind _buttoncomp (`self.ButtonComp`))
  (`VRButtonComponent.SetButtonState` _buttoncomp _lastbuttonstate false false)
  (`self.SetText` _lastbuttonstate)
  (`/Game/Platform/Interaction/Button/NativeButtonComponent.SetColor` _buttoncomp))

(fn `RunButton`
  (bind _rootcomponent (`Actor.RootComponent` (`GameplayStatics.GetPlayerCameraManager` 0)))
  (if (`self.bIsPlaying`)
    (`/Engine/EditorBlueprintResources/StandardMacros.IsValid` (`self.VoiceComponent`)
      (:`Is Valid`
        (`AudioComponent.Stop` (`self.VoiceComponent`))
        (`SceneComponent.SetVisibility` (`self.InfoWidgit`) false false)
        (`SceneComponent.SetVisibility` (`self.PrompText`) true false)
        (`self.K2_DestroyActor` (`self.SubActor`))
        (set `self.bIsPlaying` false)))
    (else
      (bind _returnvalue (`|SpawnActorFromClass` "/Game/Blueprint/Basic/BP_UMGDisplayVelo.BP_UMGDisplayVelo_C" (`KismetMathLibrary.MakeTransform` (`SceneComponent.K2_GetComponentLocation` _rootcomponent) (`SceneComponent.K2_GetComponentRotation` _rootcomponent)) "Undefined" "MultiplyWithRoot" null null))
      (set `self.SubActor` _returnvalue)
      (`|ExecutionSequence`
        (:`then_0`
          (if (not (`KismetSystemLibrary.IsDedicatedServer`))
            (`SceneComponent.SetVisibility` (`self.PrompText`) false false)
            (`SceneComponent.SetVisibility` (`self.InfoWidgit`) true false)
            (bind _aswbp_info (cast `/Game/Blueprint/Basic/WBP_Info` (`WidgetComponent.GetUserWidgetObject` (`self.InfoWidgit`))))
            (`/Game/Blueprint/Basic/WBP_Info.SetInfo` _aswbp_info (`self.InfoText`))
            (bind _returnvalue_2 (`GameplayStatics.SpawnSound2D` (`self.InfoVoice`) 1.0 1.0 0.0 null))
            (set `self.VoiceComponent` _returnvalue_2)
            (set `self.bIsPlaying` true)))
        (:`then_1`
          (`self.SetText` false))))))

(fn `UserConstructionScript`)