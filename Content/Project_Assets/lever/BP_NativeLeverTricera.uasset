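; VR lever actor that loads TriceraLevel when its VRLever component changes state and displays the current lever angle as text.
; Gripping enables Tick to refresh the text, and Tick switches itself off once the lever is released and finishes lerping.
; On a dedicated server, drop and lerp-finish events store LastAngle, whose RepNotify sets the lever angle and refreshes the text.
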(event `self.ReceiveBeginPlay`
  (`parent.ReceiveBeginPlay`))

(event `self.ReceiveTick`
  (params (DeltaSeconds :type "Float (single-precision)"))
  (`self.UpdateAngleText`) ; Sets text
  (bind (_holdingcontrollers _bisheld) (`VRGripInterface.IsHeld` (`self.VRLever`)))
  (if (not _bisheld)
    (if (not (`VRLeverComponent.bIsLerping` (`self.VRLever`)))
      (`self.SetActorTickEnabled` false))))

(event `self.VRLever.OnGripped`
  (params (GrippingController :type "GripMotionControllerComponent Object Reference") (GripInformation :type "BPActorGripInformation Structure (by ref)"))
  (`self.SetActorTickEnabled` true))

(event `self.VRLever.OnLeverStateChanged`
  (params (LeverStatus :type Boolean) (LeverStatusType :type "EVRInteractibleLeverEventType Enum" :default "LeverPositive") (LeverAngleAtTime :type "Float (single-precision)") (FullLeverAngleAtTime :type "Float (single-precision)"))
  (`GameplayStatics.OpenLevel` "TriceraLevel"))

(event `self.VRLever.OnLeverFinishedLerping`
  (params (FinalAngle :type "Float (single-precision)"))
  (if (`KismetSystemLibrary.IsDedicatedServer`)
    (set `self.LastAngle` FinalAngle)))

(event `self.VRLever.OnDropped`
  (params (GrippingController :type "GripMotionControllerComponent Object Reference") (GripInformation :type "BPActorGripInformation Structure (by ref)") (bWasSocketed :type Boolean))
  (if (`KismetSystemLibrary.IsDedicatedServer`)
    (set `self.LastAngle` (`VRLeverComponent.CurrentLeverAngle` (`self.VRLever`)))))

(fn `OnRep_LastAngle`
  (bind _vrlever (`self.VRLever`))
  (`VRLeverComponent.SetLeverAngle` _vrlever (`self.LastAngle`) (`VRLeverComponent.CurrentLeverForwardVector` _vrlever) true)
  (`self.UpdateAngleText`))

(fn `UpdateAngleText`
  (`/Engine/EditorBlueprintResources/ActorMacros.Switch Has Authority`
    (:`Authority`
      (if (`KismetSystemLibrary.IsStandalone`)
        (`TextRenderComponent.K2_SetText` (`self.Angle`) (`KismetTextLibrary.Conv_DoubleToText` (`VRLeverComponent.CurrentLeverAngle` (`self.VRLever`)) "ToZero" false true 2 324 1 1) :!label _label)))
    (:`Remote`
      (goto _label))))

(fn `UserConstructionScript`)