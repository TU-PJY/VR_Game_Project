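; BP_UMGDisplayInfo is an actor that trails the player's view in VR, apparently as a holder for subtitles or info UI.
; On BeginPlay it casts the pawn to BP_VRCharacter, enables that character's tick and its own input, and adds the VRE input mapping context.
; Each Tick, RotateSubtitles eases it toward the camera's location and yaw with VInterpTo and RInterpTo, leaving out pitch and roll.
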(event `self.ReceiveBeginPlay`
  (bind _returnvalue (`GameplayStatics.GetPlayerController` 0))
  (bind _asbp_vrcharacter (cast `/Game/Platform/Core/Character/BP_VRCharacter` (`GameplayStatics.GetPlayerPawn` 0)))
  (bind _output_get (set `self.As BP VRCharacter` _asbp_vrcharacter))
  (`self.SetActorTickEnabled` _output_get true)
  (`self.EnableInput` _returnvalue)
  (`EnhancedInputSubsystemInterface.AddMappingContext` (pcsubsystem `EnhancedInputLocalPlayerSubsystem` _returnvalue) "/Game/Platform/Input/VREInputMappingContext.VREInputMappingContext" 1 (struct)))

(event `self.ReceiveTick`
  (params (DeltaSeconds :type "Float (single-precision)"))
  (`self.RotateSubtitles` DeltaSeconds))

(fn `RotateSubtitles`
  (params (DeltaTime :type "Float (double-precision)"))
  (bind _defaultsceneroot (`self.DefaultSceneRoot`))
  (bind _transformcomponent (`PlayerCameraManager.TransformComponent` (`GameplayStatics.GetPlayerCameraManager` 0)))
  (bind (_returnvalue_roll _returnvalue_pitch _returnvalue_yaw) (`KismetMathLibrary.BreakRotator` (`KismetMathLibrary.RInterpTo` (`SceneComponent.K2_GetComponentRotation` _defaultsceneroot) (`SceneComponent.K2_GetComponentRotation` _transformcomponent) DeltaTime 2.4)))
  (`self.K2_SetActorTransform` (`KismetMathLibrary.MakeTransform` (`KismetMathLibrary.VInterpTo` (`SceneComponent.K2_GetComponentLocation` _defaultsceneroot) (`SceneComponent.K2_GetComponentLocation` _transformcomponent) DeltaTime 1.8) (`KismetMathLibrary.MakeRotator` 0.0 0.0 _returnvalue_yaw))))

(fn `UserConstructionScript`)